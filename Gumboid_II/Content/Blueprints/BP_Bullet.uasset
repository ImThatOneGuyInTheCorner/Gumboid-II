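; BP_Bullet is a projectile actor that damages what it overlaps and shows a beam trail.
; When the Bullet component begins overlapping anything other than BP_ThirdPersonCharacter, it applies fixed damage and destroys itself, printing every overlapped actor's name.
; On Trail activation, the TrailLength timeline drives the "Beam End" vector parameter.
; The construction script stores a dynamic material instance of the trail, unused in these graphs.
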(event OnComponentActivated(Trail)
  (params (Component :type Actor%20Component%20Object%20Reference) (bReset :type Boolean))
  ;[1 1 1] Bullet Trail
  (bind _newtrack_1 (Timeline|TrailLength Play)
    (:Update
      (Effects|Components|ParticleSystem|SetVectorParameter (Variables|Default|GetTrail) "Beam End" _newtrack_1))))

(event OnComponentEndOverlap(Bullet)
  (params (OverlappedComponent :type Primitive%20Component%20Object%20Reference) (OtherActor :type Actor%20Object%20Reference) (OtherComp :type Primitive%20Component%20Object%20Reference) (OtherBodyIndex :type Integer)))

(event OnComponentBeginOverlap(Bullet)
  (params (OverlappedComponent :type Primitive%20Component%20Object%20Reference) (OtherActor :type Actor%20Object%20Reference) (OtherComp :type Primitive%20Component%20Object%20Reference) (OtherBodyIndex :type Integer) (bFromSweep :type Boolean) (SweepResult :type Hit%20Result%20Structure%20%28by%20ref%29))
  ;[1 1 1] Apply Damage
  (Development|PrintString (Utilities|GetDisplayName OtherActor))
  (Utilities|Casting|CastToBP_ThirdPersonCharacter OtherActor
    (:CastFailed
      (Game|Damage|ApplyDamage OtherActor 1e+01 0 0)
      (Actor|DestroyActor))))

(event Collision|EventHit
  (params (MyComp :type Primitive%20Component%20Object%20Reference) (Other :type Actor%20Object%20Reference) (OtherComp :type Primitive%20Component%20Object%20Reference) (bSelfMoved :type Boolean) (HitLocation :type Vector :default "0, 0, 0") (HitNormal :type Vector :default "0, 0, 0") (NormalImpulse :type Vector :default "0, 0, 0") (Hit :type Hit%20Result%20Structure%20%28by%20ref%29)))

(fn ConstructionScript
  (bind _returnvalue (Rendering|Material|CreateDynamicMaterialInstance (Variables|Default|GetTrail) 0 0 "None" :!class /Script/Engine.PrimitiveComponent))
  (Variables|Default|SetTrailInstance _returnvalue))